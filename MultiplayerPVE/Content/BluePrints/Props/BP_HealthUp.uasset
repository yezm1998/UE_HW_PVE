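; BP_HealthUp is a health pickup prop built on power-up events.
; On activation it hides its static mesh, adds a fixed amount of health to the first player pawn's UserHealthComponent, and prints the resulting health on screen.
; The expire and tick events are empty, and the DestroyActor node never runs, so this graph only hides the pickup.
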(event `self.OnActivated`
  (bind _returnvalue (`self.GetComponentByClass` (`GameplayStatics.GetPlayerPawn` 0) "/Script/MultiplayerPVE.UserHealthComponent"))
  (`SceneComponent.SetVisibility` (`self.StaticMesh`) false false)
  (`UserHealthComponent.AddHealth` _returnvalue 50.0)
  (`KismetSystemLibrary.PrintString` (`KismetStringLibrary.Conv_DoubleToString` (`UserHealthComponent.Health` _returnvalue)) true true (struct :`G` 0.66 :`B` 1.0 :`A` 1.0) 5.0))

(event `self.OnExpired`)

(event `self.OnPowerUpTick`)

(fn `UserConstructionScript`)