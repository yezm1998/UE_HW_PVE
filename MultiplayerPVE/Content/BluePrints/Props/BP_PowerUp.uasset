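; Power-up prop that temporarily boosts the player pawn's swim speed, driven by activation and expiry events.
; On activation it hides its three meshes, caches the movement component's current max speed, and sets MaxSwimSpeed to double that value.
; On expiry it writes the cached speed into MaxSwimSpeed, which can differ from the original since GetMaxSpeed follows movement mode, then destroys itself.
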(event `self.OnActivated`
  (bind _returnvalue (`self.GetComponentByClass` (`GameplayStatics.GetPlayerPawn` 0) "/Script/Engine.CharacterMovementComponent"))
  (`|ExecutionSequence`
    (:`then_0`
      (`SceneComponent.SetVisibility` (`self.StaticMesh1`) false false))
    (:`then_1`
      (`SceneComponent.SetVisibility` (`self.StaticMesh2`) false false))
    (:`then_2`
      (`SceneComponent.SetVisibility` (`self.StaticMesh`) false false)
      (bind _output_get (set `self.Speed` (`MovementComponent.GetMaxSpeed` _returnvalue)))
      (bind _output_get_2 (set `CharacterMovementComponent.MaxSwimSpeed` (* 2 _output_get) _returnvalue))
      (`KismetSystemLibrary.PrintString` (`KismetStringLibrary.Conv_DoubleToString` _output_get_2) true true (struct :`G` 0.66 :`B` 1.0 :`A` 1.0) 5.0))))

(event `self.OnExpired`
  (bind _output_get (set `CharacterMovementComponent.MaxSwimSpeed` (`self.Speed`) (`self.GetComponentByClass` (`GameplayStatics.GetPlayerPawn` 0) "/Script/Engine.CharacterMovementComponent")))
  (`KismetSystemLibrary.PrintString` (`KismetStringLibrary.Conv_DoubleToString` _output_get))
  (`self.K2_DestroyActor`))

(event `self.OnPowerUpTick`)

(fn `UserConstructionScript`)