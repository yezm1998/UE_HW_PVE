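; BP_LoginControler is the lobby player controller that links each player's UI to BP_LoginGameMode.
; On BeginPlay it registers the GameInstance's PlayerInfo with the game mode, opens the WBP_GameLobby widget and requests an all-player refresh.
; Player info edits are forwarded to the game mode, while update events refresh the lobby's ready list.
; It also shows a loading widget and destroys the session to return to StartMap on leaving.
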(event `self.ReceiveBeginPlay`
  ;[1 1 1] 开始
  (`self.EVE_Init`))

(event `EVE_Init`
  ;[1 1 1] 初始化
  (bind _asbp_game_instance (cast `/Game/BluePrints/Gamemode/BP_GameInstance` (`GameplayStatics.GetGameInstance`)))
  (bind _output_get (set `self.PlayerInfo` (`/Game/BluePrints/Gamemode/BP_GameInstance.PlayerInfo` _asbp_game_instance)))
  (`self.EVE_AddplayerInfo` _output_get)
  (`self.EVE_ShowLobbyUI`))

(event `EVE_ShowLobbyUI`
  ;[1 1 1] 创建显示大厅控件
  (set `self.bShowMouseCursor` true)
  (bind _returnvalue (`|CreateWidget` "/Game/BluePrints/UI/load/WBP_GameLobby.WBP_GameLobby_C" self))
  (bind _output_get (set `self.GameLobby` _returnvalue))
  (`UserWidget.AddToViewport` _output_get 0)
  (`WidgetBlueprintLibrary.SetInputMode_GameAndUIEx` self (`self.GameLobby`))
  (`self.EVE_UpdateAllPlayer`))

(event `EVE_UpdateAllPlayer`
  ;[1 1 1] 更新所有玩家
  (bind _asbp_login_game_mode (cast `/Game/BluePrints/Gamemode/BP_LoginGameMode` (`GameplayStatics.GetGameMode`)))
  (`/Game/BluePrints/Gamemode/BP_LoginGameMode.EVE_UpdateAllPlayer` _asbp_login_game_mode))

(event `EVE_AddplayerInfo`
  (params (PlayerInfo :type "/Game/BluePrints/Pawn/PlayerInfo Structure"))
  ;[1 1 1] 添加人物信息
  (bind _asbp_login_game_mode (cast `/Game/BluePrints/Gamemode/BP_LoginGameMode` (`GameplayStatics.GetGameMode`)))
  (`/Game/BluePrints/Gamemode/BP_LoginGameMode.EVE_AddPlayerInfo` _asbp_login_game_mode PlayerInfo))

(event `EVE_UpdateSelf`
  (params (PlayerInfo :type "Array of /Game/BluePrints/Pawn/PlayerInfo Structure") (CpName :type Text) (MaxPlayerQuantity :type Integer))
  ;[1 1 1] 更新自身大厅控件信息
  (`/Game/BluePrints/UI/load/WBP_GameLobby.EVE_UpdateReady` (`self.GameLobby`) 0 PlayerInfo))

(event `EVE_ShowLoading`
  ;[1 1 1] 创建加载
  (bind _returnvalue (`|CreateWidget` "/Game/BluePrints/UI/load/WBP_LoadGame.WBP_LoadGame_C" self))
  (`UserWidget.AddToViewport` _returnvalue 0))

(event `EVE_UpdatePlayerInfo`
  (params (info :type "/Game/BluePrints/Pawn/PlayerInfo Structure"))
  ;[1 1 1] 更新玩家信息
  (bind _asbp_login_game_mode (cast `/Game/BluePrints/Gamemode/BP_LoginGameMode` (`GameplayStatics.GetGameMode`)))
  (`/Game/BluePrints/Gamemode/BP_LoginGameMode.EVE_UpdatePlayerInfo` _asbp_login_game_mode info))

(event `EVE_LeaveRomm`
  ;[1 1 1] 离开房间
  (`DestroySessionCallbackProxy.DestroySession` self
    (:`OnSuccess`
      (`KismetSystemLibrary.PrintString` "离开成功")
      (`GameplayStatics.OpenLevel` "StartMap"))
    (:`OnFailure`
      (`KismetSystemLibrary.PrintString` "离开失败"))))

(event `HideLoadUI`
  ;[1 1 1] 隐藏UI
  (set `self.GameLobby` null))

(fn `UserConstructionScript`)