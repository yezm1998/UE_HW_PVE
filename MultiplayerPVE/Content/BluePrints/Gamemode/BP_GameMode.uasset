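; Game mode Blueprint that tracks kill score and handles the end-of-game display.
; On BeginPlay it binds an actor-killed event that adds a point to the killer pawn's BP_PlayerState.
; ShowResult adds the end-game widget and stops movement on each BP_Target's LastHitBy controller.
; Enemy spawning is inactive: SpawnNewEnemy is empty, and the EQS query feeding debug-drawn BP_Target spawns is never run.
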(event `self.SpawnNewEnemy`
  ;[1 1 1] 生成NPC
)

(event `自定义事件_0`
  (params (QueryInstance :type "EnvQueryInstanceBlueprintWrapper Object Reference") (QueryStatus :type "EEnvQueryStatus Enum" :default "Processing"))
  ;[1 1 1] 生成NPC
  (switch `EEnvQueryStatus` QueryStatus
    (:`Success`
      (bind _resultlocations (`EnvQueryInstanceBlueprintWrapper.GetQueryResultsAsLocations` QueryInstance))
      (for _array_element _resultlocations
        (`KismetSystemLibrary.DrawDebugSphere` _array_element 100.0 12 (struct :`R` 0.269867 :`G` 1.0 :`B` 0.380529 :`A` 1.0) 5.0 5.0)
        (bind _returnvalue (`|SpawnActorFromClass` "/Game/BluePrints/Pawn/BP_Target.BP_Target_C" (`KismetMathLibrary.MakeTransform` _array_element) "AdjustIfPossibleButDontSpawnIfColliding" "OverrideRootScale" null null))
        (`/Game/BluePrints/Pawn/BP_Target.FindUser` _returnvalue)
        (`KismetSystemLibrary.PrintString` "create")))))

(event `self.ShowResult`
  ;[1 1 1] 结束显示
  (`|ExecutionSequence`
    (:`then_0`
      (bind _returnvalue (`|CreateWidget` "/Game/BluePrints/UI/WBP_EndGame.WBP_EndGame_C"))
      (`UserWidget.AddToViewport` _returnvalue 0))
    (:`then_1`
      (bind _outactors (`GameplayStatics.GetAllActorsOfClass` "/Game/BluePrints/Pawn/BP_Target.BP_Target_C"))
      (for _array_element _outactors
        (`Controller.StopMovement` (`Pawn.LastHitBy` _array_element))))))

(event `self.ReceiveBeginPlay`
  (add `self.OnActorKilled` (delegate `OnActorKilled_事件_0`)))

(event `OnActorKilled_事件_0` :!signature `self.OnActorKilled`
  (params (VictimActor :type "Actor Object Reference") (KillerActor :type "Actor Object Reference") (KillerActorController :type "Actor Object Reference"))
  (bind _aspawn (cast `Pawn` KillerActor))
  (bind _asbp_player_state (cast `/Game/BluePrints/Gamemode/BP_PlayerState` (`Pawn.PlayerState` _aspawn)))
  (`UserPlayerState.AddScore` _asbp_player_state 1.0))

(fn `UserConstructionScript`)