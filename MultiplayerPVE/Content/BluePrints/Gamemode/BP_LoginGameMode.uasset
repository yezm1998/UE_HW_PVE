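; BP_LoginGameMode is the multiplayer lobby game mode that tracks player controllers and info and server-travels to ThirdPersonExampleMap.
; On login the server spawns and possesses a BP_UserCharacter at the next indexed PlayerStart.
; Logouts and info updates push the player list to every BP_LoginControler.
; ShowResult opens the end-game widget and stops each BP_Target's LastHitBy; the EQS target-spawning query is left unconnected.
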(event `self.K2_OnLogout`
  (params (ExitingController :type "Controller Object Reference"))
  ;[1 1 1] 玩家退出
  (`/Engine/EditorBlueprintResources/ActorMacros.Switch Has Authority`
    (:`Authority`
      (for (_array_element _array_index) (`self.PlayerControl`)
        (if (== _array_element ExitingController)
          (`KismetArrayLibrary.Array_RemoveItem` (`self.PlayerControl`) _array_element)
          (`KismetArrayLibrary.Array_Remove` (`self.Player Info List`) _array_index)))
      (`self.EVE_UpdateAllPlayer`))))

(event `self.K2_PostLogin`
  (params (NewPlayer :type "PlayerController Object Reference"))
  ;[1 1 1] 玩家登陆
  (`/Engine/EditorBlueprintResources/ActorMacros.Switch Has Authority`
    (:`Authority`
      (`KismetArrayLibrary.Array_AddUnique` (`self.PlayerControl`) NewPlayer)
      (`self.EVE_SpawnPlayer` NewPlayer))))

(event `EVE_StartCp`
  (bind _returnvalue (`GameplayStatics.GetPlayerController` 0))
  ;[1 1 1] 场景漫游
  (bind _asbp_login_controler (cast `/Game/BluePrints/Gamemode/BP_LoginControler` _returnvalue))
  (`/Game/BluePrints/Gamemode/BP_LoginControler.HideLoadUI` _asbp_login_controler)
  (`KismetSystemLibrary.ExecuteConsoleCommand` "ServerTravel ThirdPersonExampleMap" _returnvalue))

(event `EVE_SpawnPlayer`
  (params (PC :type "PlayerController Object Reference"))
  (bind _returnvalue (`Controller.K2_GetPawn` PC))
  (bind _playerposition (`self.PlayerPosition`))
  ;[1 1 1] 生成玩家
  (`/Engine/EditorBlueprintResources/StandardMacros.IsValid` _returnvalue
    (:`Is Valid`
      (`self.K2_DestroyActor` _returnvalue))
    (:`Is Not Valid`
      _))
  (bind _outactors (`GameplayStatics.GetAllActorsOfClass` "/Script/Engine.PlayerStart"))
  (set `self.PlayerPosition` (+ _playerposition 1))
  (bind _returnvalue_2 (`|SpawnActorFromClass` "/Game/BluePrints/Pawn/BP_UserCharacter.BP_UserCharacter_C" (`KismetMathLibrary.MakeTransform` (`self.K2_GetActorLocation` (`|GetArrayItem` _outactors _playerposition))) "AdjustIfPossibleButAlwaysSpawn" "OverrideRootScale" null null))
  (`Controller.Possess` PC _returnvalue_2))

(event `EVE_AddPlayerInfo`
  (params (playerinfo :type "/Game/BluePrints/Pawn/PlayerInfo Structure (by ref)"))
  ;[1 1 1] 添加玩家信息
  (`KismetArrayLibrary.Array_AddUnique` (`self.Player Info List`) playerinfo))

(event `EVE_UpdatePlayerInfo`
  (params (info :type "/Game/BluePrints/Pawn/PlayerInfo Structure"))
  ;[1 1 1] 更新玩家属性
  (`KismetArrayLibrary.Array_Clear` (`self.TempPlayerInfoList`))
  (for _array_element (`self.Player Info List`)
    (if (`KismetTextLibrary.EqualEqual_TextText` (`KismetTextLibrary.Conv_StringToText` (`.Name_2_0FD51F4E4068336D6A3F03A8871F4AAD` (break `/Game/BluePrints/Pawn/PlayerInfo` _array_element))) (`KismetTextLibrary.Conv_StringToText` (`.Name_2_0FD51F4E4068336D6A3F03A8871F4AAD` (break `/Game/BluePrints/Pawn/PlayerInfo` info))))
      (`KismetArrayLibrary.Array_Add` (`self.TempPlayerInfoList`) info)
      (else
        (`KismetArrayLibrary.Array_Add` (`self.TempPlayerInfoList`) _array_element))))
  (set `self.Player Info List` (`self.TempPlayerInfoList`))
  (`self.EVE_UpdateAllPlayer`))

(event `EVE_UpdateAllPlayer`
  ;[1 1 1] 更新所有玩家
  (for _array_element (`self.PlayerControl`)
    (bind _asbp_login_controler (cast `/Game/BluePrints/Gamemode/BP_LoginControler` _array_element))
    (`/Game/BluePrints/Gamemode/BP_LoginControler.EVE_UpdateSelf` _asbp_login_controler (`self.Player Info List`) "" 0)))

(event `SpawnNewEnemy_1`
  ;[1 1 1] 生成NPC
)

(event `自定义事件_0`
  (params (QueryInstance :type "EnvQueryInstanceBlueprintWrapper Object Reference") (QueryStatus :type "EEnvQueryStatus Enum" :default "Processing"))
  ;[1 1 1] 生成NPC
  (switch `EEnvQueryStatus` QueryStatus
    (:`Success`
      (bind _resultlocations (`EnvQueryInstanceBlueprintWrapper.GetQueryResultsAsLocations` QueryInstance))
      (for _array_element _resultlocations
        (`KismetSystemLibrary.DrawDebugSphere` _array_element 100.0 12 (struct :`R` 0.269867 :`G` 1.0 :`B` 0.380529 :`A` 1.0) 5.0 5.0)
        (`|SpawnActorFromClass` "/Game/BluePrints/Pawn/BP_Target.BP_Target_C" (`KismetMathLibrary.MakeTransform` _array_element) "AdjustIfPossibleButDontSpawnIfColliding" "OverrideRootScale" null null)
        (`KismetSystemLibrary.PrintString` "create")))))

(event `self.ShowResult`
  (params (Success :type Boolean))
  ;[1 1 1] 结束显示
  (`|ExecutionSequence`
    (:`then_0`
      (bind _returnvalue (`|CreateWidget` "/Game/BluePrints/UI/result/WBP_EndGame.WBP_EndGame_C"))
      (`UserWidget.AddToViewport` _returnvalue 0))
    (:`then_1`
      (bind _outactors (`GameplayStatics.GetAllActorsOfClass` "/Game/BluePrints/Pawn/BP_Target.BP_Target_C"))
      (for _array_element _outactors
        (`Controller.StopMovement` (`Pawn.LastHitBy` _array_element))))))

(fn `UserConstructionScript`)