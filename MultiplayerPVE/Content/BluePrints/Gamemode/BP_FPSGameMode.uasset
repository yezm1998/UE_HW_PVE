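; FPS game mode that starts PVE mode on BeginPlay, spawns AI enemies, awards kill score and pushes end-of-match results to players.
; Melee, ranged and boss spawn events each run an EQS query and spawn at the returned locations, with debug spheres.
; Registered player controllers supply the scoreboard and result lists.
; Helper functions report whether any AI remains and whether the BP_Target NPC is alive; PVP startup is disconnected.
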(event `self.K2_PostLogin`
  (params (NewPlayer :type "PlayerController Object Reference"))
  ;[1 1 1] 玩家登陆
)

(event `自定义事件_1`
  (params (HealthComp :type "UserHealthComponent Object Reference") (Victim :type "Actor Object Reference") (Health :type "Float (double-precision)") (Damage :type "Float (double-precision)") (DamageType :type "DamageType Object Reference") (InstigatedBy :type "Controller Object Reference") (DamageCauser :type "Actor Object Reference"))
  ;[1 1 1] 开始选择游戏模式
  (bind _asbp_user_character (cast `/Game/BluePrints/Pawn/BP_UserCharacter` Victim))
  (`KismetArrayLibrary.Array_Add` (`self.TermList`) (make `/Game/BluePrints/Pawn/TermPlayInfo` (`UserCharacter.UserName` _asbp_user_character) 0 0 Health)))

(event `self.ReceiveBeginPlay`
  ;[1 1 1] 开始选择游戏模式
  (`self.PVEMode`)
  (add `self.OnActorKilled` (delegate `自定义事件_2`)))

(event `自定义事件_2` :!signature `self.OnActorKilled`
  (params (VictimActor :type "Actor Object Reference") (VictimActorController :type "Actor Object Reference") (KillerActor :type "Actor Object Reference") (KillerActorController :type "Actor Object Reference"))
  ;[1 1 1] 开始选择游戏模式
  (bind _asbp_controler (cast `/Game/BluePrints/Gamemode/BP_Controler` KillerActorController)
    (:`then`
      (`/Game/BluePrints/Gamemode/BP_Controler.Add Score` _asbp_controler))
    (:`CastFailed`
      (bind _asbp_user_character (cast `/Game/BluePrints/Pawn/BP_UserCharacter` KillerActorController))
      (bind _asbp_controler_2 (cast `/Game/BluePrints/Gamemode/BP_Controler` (`Pawn.GetController` _asbp_user_character)))
      (`/Game/BluePrints/Gamemode/BP_Controler.Add Score` _asbp_controler_2))))

(event `EVE_AddPlayerInfo`
  (params (playerinfo :type "/Game/BluePrints/Gamemode/BP_Controler Object Reference (by ref)"))
  ;[1 1 1] 添加玩家信息
  (`KismetArrayLibrary.Array_Add` (`self.Player Controler List`) playerinfo))

(event `self.PVPEndGame`
  ;[1 1 1] 结束显示
)

(event `self.ShowResult`
  (params (Success :type Boolean))
  (bind _player_controler_list (`self.Player Controler List`))
  ;[1 1 1] 结束显示
  (for _array_element _player_controler_list
    (bind _asuser_player_state (cast `UserPlayerState` (`Controller.PlayerState` _array_element)))
    (`KismetArrayLibrary.Array_Add` (`self.Result`) (make `/Game/BluePrints/Pawn/PlayerResult` (`UserPlayerState.NumberDied` _asuser_player_state) (`/Game/BluePrints/Gamemode/BP_Controler.Socre` _array_element) (`.Name_2_0FD51F4E4068336D6A3F03A8871F4AAD` (break `/Game/BluePrints/Pawn/PlayerInfo` (`/Game/BluePrints/Gamemode/BP_Controler.PlayerInfo` _array_element))))))
  (for _array_element_2 _player_controler_list
    (`/Game/BluePrints/Gamemode/BP_Controler.ShowResult` _array_element_2 (`self.Result`) Success)))

(event `self.SpawnNewMeleeEnemy`
  ;[1 1 1] 生成近战
  (bind _returnvalue (`EnvQueryManager.RunEQSQuery` "/Game/AI/EQS_AISpawn.EQS_AISpawn" self "RandomBest25Pct"))
  (add `EnvQueryInstanceBlueprintWrapper.OnQueryFinishedEvent` _returnvalue (delegate `自定义事件_0`)))

(event `自定义事件_0`
  (params (QueryInstance :type "EnvQueryInstanceBlueprintWrapper Object Reference") (QueryStatus :type "EEnvQueryStatus Enum" :default "Processing"))
  ;[1 1 1] 生成近战
  (switch `EEnvQueryStatus` QueryStatus
    (:`Success`
      (bind _resultlocations (`EnvQueryInstanceBlueprintWrapper.GetQueryResultsAsLocations` QueryInstance))
      (for _array_element _resultlocations
        (`KismetSystemLibrary.DrawDebugSphere` _array_element 100.0 12 (struct :`R` 0.269867 :`G` 1.0 :`B` 0.380529 :`A` 1.0) 5.0 5.0)
        (`|SpawnActorFromClass` "/Game/BluePrints/Pawn/BP_UserCharacter_Melee.BP_UserCharacter_Melee_C" (`KismetMathLibrary.MakeTransform` _array_element) "AdjustIfPossibleButDontSpawnIfColliding" "OverrideRootScale" null null)))))

(event `self.SpawnNewRemoteEnemy`
  ;[1 1 1] 生成远程
  (bind _returnvalue (`EnvQueryManager.RunEQSQuery` "/Game/AI/EQS_AISpawn.EQS_AISpawn" self "RandomBest25Pct"))
  (add `EnvQueryInstanceBlueprintWrapper.OnQueryFinishedEvent` _returnvalue (delegate `CustomEvent1`)))

(event `CustomEvent1`
  (params (QueryInstance :type "EnvQueryInstanceBlueprintWrapper Object Reference") (QueryStatus :type "EEnvQueryStatus Enum" :default "Processing"))
  ;[1 1 1] 生成远程
  (switch `EEnvQueryStatus` QueryStatus
    (:`Success`
      (bind _resultlocations (`EnvQueryInstanceBlueprintWrapper.GetQueryResultsAsLocations` QueryInstance))
      (for _array_element _resultlocations
        (`KismetSystemLibrary.DrawDebugSphere` _array_element 100.0 12 (struct :`R` 0.269867 :`G` 1.0 :`B` 0.380529 :`A` 1.0) 5.0 5.0)
        (`|SpawnActorFromClass` "/Game/BluePrints/Pawn/BP_UserCharacter_Remote.BP_UserCharacter_Remote_C" (`KismetMathLibrary.MakeTransform` _array_element) "AdjustIfPossibleButDontSpawnIfColliding" "OverrideRootScale" null null)))))

(event `self.SpawnNewBossEnemy`
  ;[1 1 1] 生成boss
  (bind _returnvalue (`EnvQueryManager.RunEQSQuery` "/Game/AI/EQS_AISpawn.EQS_AISpawn" self "RandomBest25Pct"))
  (add `EnvQueryInstanceBlueprintWrapper.OnQueryFinishedEvent` _returnvalue (delegate `CustomEvent`)))

(event `CustomEvent`
  (params (QueryInstance :type "EnvQueryInstanceBlueprintWrapper Object Reference") (QueryStatus :type "EEnvQueryStatus Enum" :default "Processing"))
  ;[1 1 1] 生成boss
  (switch `EEnvQueryStatus` QueryStatus
    (:`Success`
      (bind _resultlocations (`EnvQueryInstanceBlueprintWrapper.GetQueryResultsAsLocations` QueryInstance))
      (for _array_element _resultlocations
        (`KismetSystemLibrary.DrawDebugSphere` _array_element 100.0 12 (struct :`R` 0.269867 :`G` 1.0 :`B` 0.380529 :`A` 1.0) 5.0 5.0)
        (`|SpawnActorFromClass` "/Game/BluePrints/Pawn/BP_UserCharacter_Boss.BP_UserCharacter_Boss_C" (`KismetMathLibrary.MakeTransform` _array_element) "AdjustIfPossibleButDontSpawnIfColliding" "OverrideRootScale" null null)))))

(fn `CheckAllAI`
  (returns (ReturnValue :type Boolean))
  (bind _outactors (`GameplayStatics.GetAllActorsOfClass` "/Game/BluePrints/Pawn/BP_UserCharacter_Melee.BP_UserCharacter_Melee_C"))
  (bind _outactors_2 (`GameplayStatics.GetAllActorsOfClass` "/Game/BluePrints/Pawn/BP_UserCharacter_Remote.BP_UserCharacter_Remote_C"))
  (bind _outactors_3 (`GameplayStatics.GetAllActorsOfClass` "/Game/BluePrints/Pawn/BP_UserCharacter_Boss.BP_UserCharacter_Boss_C"))
  (return (> (+ (`KismetArrayLibrary.Array_Length` _outactors) (`KismetArrayLibrary.Array_Length` _outactors_2) (`KismetArrayLibrary.Array_Length` _outactors_3)) 0)))

(fn `CheckNPCAlive`
  (returns (ReturnValue :type Boolean))
  (bind _outactors (`GameplayStatics.GetAllActorsOfClass` "/Game/BluePrints/Pawn/BP_Target.BP_Target_C"))
  (if (> (`KismetArrayLibrary.Array_Length` _outactors) 0)
    (return (> (`/Game/BluePrints/Pawn/BP_Target.Health` (`|GetArrayItem` _outactors)) 0.0))
    (else
      (return true))))

(fn `Get Controller List`
  (returns (NewParam :type "Array of /Game/BluePrints/Pawn/TermPlayInfo Structure"))
  (`KismetArrayLibrary.Array_Clear` (`self.TermList`))
  (for _array_element (`self.Player Controler List`)
    (bind _asuser_player_state (cast `UserPlayerState` (`Controller.PlayerState` _array_element)))
    (bind _asbp_user_character (cast `/Game/BluePrints/Pawn/BP_UserCharacter` (`Controller.K2_GetPawn` _array_element)))
    (bind _returnvalue (`UserCharacter.GetHealth` _asbp_user_character))
    (`KismetArrayLibrary.Array_Add` (`self.TermList`) (make `/Game/BluePrints/Pawn/TermPlayInfo` (`.Name_2_0FD51F4E4068336D6A3F03A8871F4AAD` (break `/Game/BluePrints/Pawn/PlayerInfo` (`/Game/BluePrints/Gamemode/BP_Controler.PlayerInfo` _array_element))) (`/Game/BluePrints/Gamemode/BP_Controler.Socre` _array_element) (`UserPlayerState.NumberDied` _asuser_player_state) _returnvalue)))
  (return (`self.TermList`)))

(fn `UserConstructionScript`)