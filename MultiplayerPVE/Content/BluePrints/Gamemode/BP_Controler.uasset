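; Player controller for the FPS game's PVP and PVE modes, handling player registration, score and match UI.
; On init it reads player info from the game instance, shows the lobby widget and registers with BP_FPSGameMode.
; It builds a match result from score, name and deaths for UpdateOnServer, and shows win or lose screens.
; It also caches the controller list, plus prep time and wave number from PVEGameModeBase.
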(event `self.ReceiveBeginPlay`
  ;[1 1 1] 开始
  (`self.EVE_Init`))

(event `EVE_Init`
  ;[1 1 1] 初始化
  (bind _asbp_game_instance (cast `/Game/BluePrints/Gamemode/BP_GameInstance` (`GameplayStatics.GetGameInstance`) :!label _label))
  (bind _playerinfo (`/Game/BluePrints/Gamemode/BP_GameInstance.PlayerInfo` _asbp_game_instance))
  (`KismetSystemLibrary.PrintString` (`.Name_2_0FD51F4E4068336D6A3F03A8871F4AAD` (break `/Game/BluePrints/Pawn/PlayerInfo` _playerinfo)))
  (`self.EVE_ShowLobbyUI`)
  (`self.EVE_AddplayerInfo` self _playerinfo)
  (`GameplayStatics.SetViewportMouseCaptureMode` "CapturePermanently"))

(event `EVE_AddplayerInfo`
  (params (controller :type "/Game/BluePrints/Gamemode/BP_Controler Object Reference") (info :type "/Game/BluePrints/Pawn/PlayerInfo Structure"))
  ;[1 1 1] 添加人物信息
  (set `self.PlayerInfo` info)
  (bind _asbp_fpsgame_mode (cast `/Game/BluePrints/Gamemode/BP_FPSGameMode` (`GameplayStatics.GetGameMode`)))
  (`/Game/BluePrints/Gamemode/BP_FPSGameMode.EVE_AddPlayerInfo` _asbp_fpsgame_mode controller))

(event `ServerInit`
  ;[1 1 1] 初始化
  (goto _label))

(event `EVE_ShowLobbyUI`
  ;[1 1 1] 创建显示大厅控件
  (bind _returnvalue (`|CreateWidget` "/Game/BluePrints/UI/WBP_UserInfo.WBP_UserInfo_C" self))
  (bind _output_get (set `self.UserInfo` _returnvalue))
  (`UserWidget.AddToViewport` _output_get 0))

(event `GetClientResult`
  (bind _result (`self.Get One Result`))
  (`self.UpdateOnServer` _result))

(event `ShowResult`
  (params (PlayerList :type "Array of /Game/BluePrints/Pawn/PlayerResult Structure") (success :type Boolean))
  ;[1 1 1] PVP结果显示
  (set `self.bShowMouseCursor` true)
  (if success
    (bind _returnvalue (`|CreateWidget` "/Game/BluePrints/UI/result/WBP_PVPEndGame.WBP_PVPEndGame_C" self))
    (bind _output_get (set `self.PVPend` _returnvalue))
    (`/Game/BluePrints/UI/result/WBP_PVPEndGame.show` _output_get PlayerList)
    (`UserWidget.AddToViewport` _output_get 0)
    (else
      (bind _returnvalue_2 (`|CreateWidget` "/Game/BluePrints/UI/result/WBP_PVPEndGameLose.WBP_PVPEndGameLose_C" self))
      (bind _output_get_2 (set `self.NewVar_0` _returnvalue_2))
      (`/Game/BluePrints/UI/result/WBP_PVPEndGameLose.show` _output_get_2 PlayerList)
      (`UserWidget.AddToViewport` _output_get_2 0))))

(event `UpdateOnServer`
  (params (NewParam :type "/Game/BluePrints/Pawn/PlayerResult Structure"))
  (bind _output_get (set `self.ThisResult` NewParam))
  (`KismetSystemLibrary.PrintString` (`.Name_5_A8ACB4F946F19BD16FF434A7565FA61E` (break `/Game/BluePrints/Pawn/PlayerResult` _output_get))))

(event `Add Score`
  ;[1 1 1] 加分
  (set `self.Socre` (+ (`self.Socre`) 1)))

(event `GetTermInfo`
  ;[1 1 1] 获取团队信息
  (bind _asbp_fpsgame_mode (cast `/Game/BluePrints/Gamemode/BP_FPSGameMode` (`GameplayStatics.GetGameMode`)))
  (bind _newparam (`/Game/BluePrints/Gamemode/BP_FPSGameMode.Get Controller List` _asbp_fpsgame_mode))
  (set `self.TermList` _newparam))

(event `ReadyTime`
  (bind _aspvegame_mode_base (cast `PVEGameModeBase` (`GameplayStatics.GetGameMode`)))
  (set `self.PrepareTime` (`PVEGameModeBase.PrepareTime` _aspvegame_mode_base)))

(event `GetWave`
  (bind _aspvegame_mode_base (cast `PVEGameModeBase` (`GameplayStatics.GetGameMode`)))
  (set `self.WaveNum` (`KismetMathLibrary.Conv_Int64ToInt` (`PVEGameModeBase.WaveNumber` _aspvegame_mode_base))))

(event `HideLoadUI`
  ;[1 1 1] 隐藏UI
)

(fn `Get One Result`
  (returns (result :type "/Game/BluePrints/Pawn/PlayerResult Structure"))
  (bind _asbp_player_state (cast `/Game/BluePrints/Gamemode/BP_PlayerState` (`self.PlayerState`))
    (:`then`
      (return (make `/Game/BluePrints/Pawn/PlayerResult` (`UserPlayerState.NumberDied` _asbp_player_state) (`self.Socre`) (`.Name_2_0FD51F4E4068336D6A3F03A8871F4AAD` (break `/Game/BluePrints/Pawn/PlayerInfo` (`self.PlayerInfo`))))))
    (:`CastFailed`
      (return))))

(fn `Gettime`
  (returns (NewParam :type Integer))
  (return (`self.PrepareTime`)))

(fn `Getwavenum`
  (returns (NewParam :type Integer))
  (return (`self.WaveNum`)))

(fn `UserConstructionScript`)