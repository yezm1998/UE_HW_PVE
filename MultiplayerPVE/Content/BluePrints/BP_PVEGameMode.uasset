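; BP_PVEGameMode is a PVE game mode that spawns BP_Target enemies and displays the end-game screen.
; SpawnNewEnemy runs the EQS_AI query, spawns a target at each returned location with collision adjustment, and calls FindUser on it.
; ShowResult adds the WBP_EndGame widget to the viewport.
; BeginPlay is empty, and leftover stop-movement and debug-sphere nodes are disconnected.
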(event `self.ReceiveBeginPlay`)

(event `self.SpawnNewEnemy`
  ;[1 1 1] 生成NPC
  (bind _returnvalue (`EnvQueryManager.RunEQSQuery` "/Game/AI/EQS_AI.EQS_AI" self "RandomBest25Pct"))
  (add `EnvQueryInstanceBlueprintWrapper.OnQueryFinishedEvent` _returnvalue (delegate `自定义事件_0`)))

(event `自定义事件_0`
  (params (QueryInstance :type "EnvQueryInstanceBlueprintWrapper Object Reference") (QueryStatus :type "EEnvQueryStatus Enum" :default "Processing"))
  ;[1 1 1] 生成NPC
  (switch `EEnvQueryStatus` QueryStatus
    (:`Success`
      (bind _resultlocations (`EnvQueryInstanceBlueprintWrapper.GetQueryResultsAsLocations` QueryInstance))
      (for _array_element _resultlocations
        (bind _returnvalue (`|SpawnActorFromClass` "/Game/BluePrints/Pawn/BP_Target.BP_Target_C" (`KismetMathLibrary.MakeTransform` _array_element) "AdjustIfPossibleButDontSpawnIfColliding" "OverrideRootScale" null null))
        (`/Game/BluePrints/Pawn/BP_Target.FindUser` _returnvalue)
        (`KismetSystemLibrary.PrintString` "create")))))

(event `self.ShowResult`
  ;[1 1 1] 结束显示
  (bind _returnvalue (`|CreateWidget` "/Game/BluePrints/UI/WBP_EndGame.WBP_EndGame_C"))
  (`UserWidget.AddToViewport` _returnvalue 0))

(fn `UserConstructionScript`)