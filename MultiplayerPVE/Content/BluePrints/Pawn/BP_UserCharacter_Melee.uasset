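; Melee AI character pawn that can drop pickups for supplies.
; On BeginPlay it starts the BT_MeleeAI behavior tree on its AI controller and registers itself as the User of its WBP_AI widget.
; The SuppliesDrop event makes cascading random rolls to spawn a power-up, a health-up or nothing at the given location, marking any drop with a debug sphere.
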(event `self.ReceiveTick`
  (params (DeltaSeconds :type "Float (single-precision)"))
  (`parent.ReceiveTick` DeltaSeconds))

(event `self.ReceiveBeginPlay`
  ;[1 1 1] 找人
  (`parent.ReceiveBeginPlay`)
  (`AIController.RunBehaviorTree` (`AIBlueprintHelperLibrary.GetAIController` self) "/Game/AI/BT_MeleeAI.BT_MeleeAI")
  (bind _aswbp_ai (cast `/Game/BluePrints/UI/WBP_AI` (`WidgetComponent.GetUserWidgetObject` (`self.Widget`))))
  (set `/Game/BluePrints/UI/WBP_AI.user` self _aswbp_ai))

(event `self.SuppliesDrop`
  (params (Location :type "Vector Structure"))
  (bind _returnvalue (`KismetMathLibrary.RandomInteger` 10))
  (if (< _returnvalue 3)
    (`|SpawnActorFromClass` "/Game/BluePrints/Props/BP_PickUp_Powerup.BP_PickUp_Powerup_C" (`KismetMathLibrary.MakeTransform` Location) "AlwaysSpawn" "OverrideRootScale" null null)
    (`KismetSystemLibrary.DrawDebugSphere` Location 100.0 12 (struct :`R` 0.269867 :`G` 1.0 :`B` 0.380529 :`A` 1.0) 5.0 5.0 :!label _label)
    (elif (< _returnvalue 6)
      (`|SpawnActorFromClass` "/Game/BluePrints/Props/BP_PickUp_Healthup.BP_PickUp_Healthup_C" (`KismetMathLibrary.MakeTransform` Location) "AlwaysSpawn" "OverrideRootScale" null null)
      (goto _label))))

(fn `UserConstructionScript`
  (`parent.UserConstructionScript`))