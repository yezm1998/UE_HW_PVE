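; AI-controlled "Remote" character pawn that can drop weapon pickups as supplies.
; On BeginPlay it runs the BT_RemoteAI behavior tree and hands itself to its WBP_AI widget as the user.
; SuppliesDrop makes chained random rolls to spawn an AK47, a launcher or nothing at the given location.
; Leftover target search, blackboard and debug-draw nodes are disconnected.
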(event `self.ReceiveBeginPlay`
  ;[1 1 1] 找人
  (`parent.ReceiveBeginPlay`)
  (`AIController.RunBehaviorTree` (`AIBlueprintHelperLibrary.GetAIController` self) "/Game/AI/BT_RemoteAI.BT_RemoteAI")
  (bind _aswbp_ai (cast `/Game/BluePrints/UI/WBP_AI` (`WidgetComponent.GetUserWidgetObject` (`self.Widget`))))
  (set `/Game/BluePrints/UI/WBP_AI.user` self _aswbp_ai))

(event `self.SuppliesDrop`
  (params (Location :type "Vector Structure"))
  (bind _returnvalue (`KismetMathLibrary.RandomInteger` 10))
  (if (< _returnvalue 3)
    (`|SpawnActorFromClass` "/Game/BluePrints/Pawn/BP_UserWeapon_AK47.BP_UserWeapon_AK47_C" (`KismetMathLibrary.MakeTransform` Location) "AlwaysSpawn" "OverrideRootScale" null null)
    (elif (< _returnvalue 6)
      (`|SpawnActorFromClass` "/Game/BluePrints/Pawn/BP_WeaponLauncher.BP_WeaponLauncher_C" (`KismetMathLibrary.MakeTransform` Location) "AlwaysSpawn" "OverrideRootScale" null null))))

(fn `UserConstructionScript`
  (`parent.UserConstructionScript`))