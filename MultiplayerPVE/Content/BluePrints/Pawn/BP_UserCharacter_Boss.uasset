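; Boss character pawn that runs on AI, spawns venom traps and can drop a weapon as supplies.
; BeginPlay starts the BT_BossAI behavior tree on its AI controller and hands itself to the WBP_AI widget as its user.
; BossFire spawns a short-lived BP_VenomTrap at a supplied transform.
; SuppliesDrop spawns an M4A1 weapon at a given location and marks it with a debug sphere.
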(event `BossFire`
  (params (NewParam :type "Transform Structure"))
  (bind _returnvalue (`|SpawnActorFromClass` "/Game/BluePrints/Props/BP_VenomTrap.BP_VenomTrap_C" NewParam "AlwaysSpawn" "OverrideRootScale" null null))
  (`self.SetLifeSpan` _returnvalue 3.0))

(event `self.ReceiveBeginPlay`
  ;[1 1 1] 找人
  (`parent.ReceiveBeginPlay`)
  (`AIController.RunBehaviorTree` (`AIBlueprintHelperLibrary.GetAIController` self) "/Game/AI/BT_BossAI.BT_BossAI")
  (bind _aswbp_ai (cast `/Game/BluePrints/UI/WBP_AI` (`WidgetComponent.GetUserWidgetObject` (`self.Widget`))))
  (set `/Game/BluePrints/UI/WBP_AI.user` self _aswbp_ai))

(event `self.SuppliesDrop`
  (params (Location :type "Vector Structure"))
  (`|SpawnActorFromClass` "/Game/BluePrints/Pawn/BP_UserWeapon_M4A1.BP_UserWeapon_M4A1_C" (`KismetMathLibrary.MakeTransform` Location) "AlwaysSpawn" "OverrideRootScale" null null)
  (`KismetSystemLibrary.DrawDebugSphere` Location 100.0 12 (struct :`R` 0.269867 :`G` 1.0 :`B` 0.380529 :`A` 1.0) 5.0 5.0))

(fn `UserConstructionScript`
  (`parent.UserConstructionScript`))