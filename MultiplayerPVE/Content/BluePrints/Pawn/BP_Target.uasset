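; BP_Target is an NPC target character that turns to face the player and awards score when killed.
; Radial damage lowers Health and updates its WBP_NPC widget; at zero it disables collision, stops movement, increments the GameInstance PlayerInfo score and expires after a delay.
; Tick sets yaw toward the player while alive, using RInterpTo with a constant delta time.
; Point damage is empty, and behavior tree startup and player-damage logic are disconnected.
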(event `self.ReceiveBeginPlay`
  ;[1 1 1] 找人
)

(event `self.ReceiveRadialDamage`
  (params (DamageReceived :type "Float (single-precision)") (DamageType :type "DamageType Object Reference") (Origin :type "Vector Structure") (HitInfo :type "HitResult Structure (by ref)") (InstigatedBy :type "Controller Object Reference") (DamageCauser :type "Actor Object Reference"))
  (bind _output_get (set `self.Health` (- (`self.Health`) DamageReceived)))
  (bind _aswbp_npc (cast `/Game/BluePrints/UI/WBP_NPC` (`WidgetComponent.GetUserWidgetObject` (`self.Widget`))))
  (set `/Game/BluePrints/UI/WBP_NPC.NpcHealth` _output_get _aswbp_npc)
  (if (not (> _output_get 0.0))
    (set `self.bDied` true)
    (`PrimitiveComponent.SetCollisionEnabled` (`self.CapsuleComponent`) "NoCollision")
    (`MovementComponent.StopMovementImmediately` (`self.CharacterMovement`))
    (bind _asbp_game_instance (cast `/Game/BluePrints/Gamemode/BP_GameInstance` (`GameplayStatics.GetGameInstance`)))
    (bind (_name _state _score) (break `/Game/BluePrints/Pawn/PlayerInfo` (`/Game/BluePrints/Gamemode/BP_GameInstance.PlayerInfo` _asbp_game_instance)))
    (set `/Game/BluePrints/Gamemode/BP_GameInstance.PlayerInfo` (make `/Game/BluePrints/Pawn/PlayerInfo` _name _state (`KismetMathLibrary.Conv_Int64ToInt` (`KismetMathLibrary.Conv_IntToInt64` (+ _score 1)))) _asbp_game_instance)
    (`self.SetLifeSpan` 5.0)))

(event `self.UserHealth.OnHealthChanged`
  (params (HealthComp :type "UserHealthComponent Object Reference") (Health :type "Float (single-precision)") (Damage :type "Float (single-precision)") (DamageType :type "DamageType Object Reference") (InstigatedBy :type "Controller Object Reference") (DamageCauser :type "Actor Object Reference"))
  ;[1 1 1] 扣血
)

(event `self.ReceivePointDamage`
  (params (Damage :type "Float (single-precision)") (DamageType :type "DamageType Object Reference") (HitLocation :type "Vector Structure") (HitNormal :type "Vector Structure") (HitComponent :type "PrimitiveComponent Object Reference") (BoneName :type Name) (ShotFromDirection :type "Vector Structure") (InstigatedBy :type "Controller Object Reference") (DamageCauser :type "Actor Object Reference") (HitInfo :type "HitResult Structure (by ref)"))
  ;[1 1 1] 扣血
)

(event `self.ReceiveTick`
  (params (DeltaSeconds :type "Float (single-precision)"))
  (bind _returnvalue (`GameplayStatics.GetPlayerCharacter` 0))
  (bind (_returnvalue_roll _returnvalue_pitch _returnvalue_yaw) (`KismetMathLibrary.BreakRotator` (`KismetMathLibrary.RInterpTo` (`self.K2_GetActorRotation`) (`KismetMathLibrary.FindLookAtRotation` (`self.K2_GetActorLocation`) (`self.K2_GetActorLocation` _returnvalue)) 1.0 1.0)))
  ;[1 1 1] 朝向
  (`/Engine/EditorBlueprintResources/StandardMacros.IsValid` _returnvalue
    (:`Is Valid`
      (if (> (`self.Health`) 0.0)
        (`self.K2_SetActorRotation` (`KismetMathLibrary.MakeRotator` 0.0 0.0 _returnvalue_yaw))))))

(fn `UserConstructionScript`)

(fn `新函数_0`)