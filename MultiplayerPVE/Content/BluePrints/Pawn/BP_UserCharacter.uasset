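; BP_UserCharacter is the player character Blueprint, which creates the user info HUD widget and sets game-only input on BeginPlay.
; Left mouse press and release start and stop attack montages chosen by the current weapon type, as a fire test.
; The first weapon type picks a running or standing Box montage by velocity, while the other two share a rifle hip-fire montage.
; Q plays a pistol equip montage and prints a debug string.
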(event `self.ReceiveBeginPlay`
  ;[1 1 1] 创建角色UI
  (bind _returnvalue (`|CreateWidget` "/Game/BluePrints/UI/WBP_UserInfo.WBP_UserInfo_C" (`GameplayStatics.GetPlayerController` 0)))
  (`UserWidget.AddToViewport` _returnvalue 0)
  (`WidgetBlueprintLibrary.SetInputMode_GameOnly` (`GameplayStatics.GetPlayerController` 0)))

(event `Key|LeftMouseButton`
  (params (Key :type "Key Structure"))
  (bind _returnvalue (`SkeletalMeshComponent.GetAnimInstance` (`self.Mesh`)))
  (bind _returnvalue_2 (`SkeletalMeshComponent.GetAnimInstance` (`self.Mesh`)))
  (bind _returnvalue_3 (`SkeletalMeshComponent.GetAnimInstance` (`self.Mesh`)))
  (bind _thisweapontype (`UserWeapon.ThisWeaponType` (`self.MyWeapon`)))
  (bind _returnvalue_4 (> (`KismetMathLibrary.VSize` (`self.GetVelocity`)) 10.0))
  ;[1 1 1] 开火测试
  (:`Pressed`
    (switch `WeaponType` _thisweapontype
      (:`Dagger`
        (if _returnvalue_4
          (`AnimInstance.Montage_Play` _returnvalue "/Game/AnimStarterPack/Box_Anim_mixamo_Run.Box_Anim_mixamo_Run" 1.0 "MontageLength" 0.0 true)
          (else
            (`AnimInstance.Montage_Play` _returnvalue "/Game/AnimStarterPack/Box_Montage.Box_Montage" 1.0 "MontageLength" 0.0 true))))
      (:`Gun`
        (`AnimInstance.Montage_Play` _returnvalue_3 "/Game/AnimStarterPack/Fire_Rifle_Hip_Montage.Fire_Rifle_Hip_Montage" 1.0 "MontageLength" 0.0 true))
      (:`Grenade`
        (`AnimInstance.Montage_Play` _returnvalue_2 "/Game/AnimStarterPack/Fire_Rifle_Hip_Montage.Fire_Rifle_Hip_Montage" 1.0 "MontageLength" 0.0 true))))
  (:`Released`
    (switch `WeaponType` _thisweapontype
      (:`Dagger`
        (if _returnvalue_4
          (`AnimInstance.Montage_Stop` _returnvalue 0.0 "/Game/AnimStarterPack/Box_Anim_mixamo_Run.Box_Anim_mixamo_Run")
          (else
            (`AnimInstance.Montage_Stop` _returnvalue 0.0 "/Game/AnimStarterPack/Box_Montage.Box_Montage"))))
      (:`Gun`
        (`AnimInstance.Montage_Stop` _returnvalue_3 0.0 "/Game/AnimStarterPack/Fire_Rifle_Hip_Montage.Fire_Rifle_Hip_Montage"))
      (:`Grenade`
        (`AnimInstance.Montage_Stop` _returnvalue_2 0.0 "/Game/AnimStarterPack/Fire_Rifle_Hip_Montage.Fire_Rifle_Hip_Montage")))))

(event `Key|Q`
  (params (Key :type "Key Structure"))
  (:`Pressed`
    (`AnimInstance.Montage_Play` (`SkeletalMeshComponent.GetAnimInstance` (`self.Mesh`)) "/Game/AnimStarterPack/Equip_Pistol_Standing_Montage.Equip_Pistol_Standing_Montage" 1.0 "MontageLength" 0.0 true)
    (`KismetSystemLibrary.PrintString` "tab")))

(fn `UserConstructionScript`)