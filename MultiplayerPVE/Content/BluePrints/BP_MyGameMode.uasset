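; BP_MyGameMode is a game mode Blueprint that spawns BP_Target NPCs at locations chosen by the Environment Query System.
; Its SpawnNPC event runs the EQS_AI query on itself in random-best-25% mode and binds a callback to query completion.
; On success, each returned location gets a temporary debug sphere and a spawned BP_Target, unless collision prevents it, on which FindUser is then called.
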(event `SpawnNPC`
  (bind _returnvalue (`EnvQueryManager.RunEQSQuery` "/Game/AI/EQS_AI.EQS_AI" self "RandomBest25Pct"))
  (add `EnvQueryInstanceBlueprintWrapper.OnQueryFinishedEvent` _returnvalue (delegate `自定义事件_0`)))

(event `自定义事件_0`
  (params (QueryInstance :type "EnvQueryInstanceBlueprintWrapper Object Reference") (QueryStatus :type "EEnvQueryStatus Enum" :default "Processing"))
  (switch `EEnvQueryStatus` QueryStatus
    (:`Success`
      (bind _resultlocations (`EnvQueryInstanceBlueprintWrapper.GetQueryResultsAsLocations` QueryInstance))
      (for _array_element _resultlocations
        (`KismetSystemLibrary.DrawDebugSphere` _array_element 100.0 12 (struct :`R` 0.269867 :`G` 1.0 :`B` 0.380529 :`A` 1.0) 5.0 5.0)
        (bind _returnvalue (`|SpawnActorFromClass` "/Game/BluePrints/Pawn/BP_Target.BP_Target_C" (`KismetMathLibrary.MakeTransform` _array_element) "AdjustIfPossibleButDontSpawnIfColliding" "OverrideRootScale" null null))
        (`/Game/BluePrints/Pawn/BP_Target.FindUser` _returnvalue)))))

(fn `UserConstructionScript`)