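; Behavior tree node that picks the target for an AI-controlled BP_UserCharacter and writes it to a blackboard key.
; On each AI tick it keeps the character's current Target while that is valid and its truncated health is above zero.
; Otherwise it falls back to the first BP_Target found in the level, with no distance, health or empty-list check.
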(event `self.ReceiveTickAI`
  (params (OwnerController :type "AIController Object Reference") (ControlledPawn :type "Pawn Object Reference") (DeltaSeconds :type "Float (single-precision)"))
  (bind _asbp_user_character (cast `/Game/BluePrints/Pawn/BP_UserCharacter` ControlledPawn))
  (bind _target (`/Game/BluePrints/Pawn/BP_UserCharacter.Target` _asbp_user_character))
  (`/Engine/EditorBlueprintResources/StandardMacros.IsValid` _target
    (:`Is Valid`
      (bind _returnvalue (`UserCharacter.GetHealth` _target))
      (if (> (`KismetMathLibrary.FTrunc` _returnvalue) 0)
        (`BTFunctionLibrary.SetBlackboardValueAsObject` (`self.Blackboard`) _target)
        (else
          (bind _outactors (`GameplayStatics.GetAllActorsOfClass` "/Game/BluePrints/Pawn/BP_Target.BP_Target_C" :!label _label))
          (`BTFunctionLibrary.SetBlackboardValueAsObject` (`self.Blackboard`) (`|GetArrayItem` _outactors)))))
    (:`Is Not Valid`
      (goto _label))))